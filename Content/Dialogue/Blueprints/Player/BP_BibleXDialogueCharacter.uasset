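; BP_BibleXDialogueCharacter is a first-person player character that starts dialogue with actors in front of it.
; Pressing Interact traces from the first-person camera along its forward vector out to DialogueTraceDistance.
; The BibleXDialogueOrigin component's TryStartDialogue runs the trace, with debug line drawing on, and begins dialogue if it finds an actor with the proper component.
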(event Input|ActionEvents|InputActionInteract
  (params (Key :type Key%20Structure :default "None"))
  (:Pressed
    ;[1 1 1] Try starting Dialogue by casting out from in front of player, will begin dialogue immediately if actor with proper component is found
    (Class|BibleXDialogueOriginComponent|TryStartDialogue (Variables|Default|GetBibleXDialogueOrigin) (Transformation|GetWorldLocation (Variables|Default|GetFirstPersonCameraComponent)) (+ (Transformation|GetWorldLocation (Variables|Default|GetFirstPersonCameraComponent)) (* (Math|Vector|GetForwardVector (Variables|Default|GetFirstPersonCameraComponent)) (Variables|Dialogue|GetDialogueTraceDistance))) true)))

(fn ConstructionScript)