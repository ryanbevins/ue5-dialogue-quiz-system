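; Quiz-style dialogue NPC that asks questions with adaptive difficulty through its BibleXDialogueTarget component.
; BeginDialogue draws and removes an entry within the current difficulty limit, shows it in WBP_DialogueMain with UI-only input and plays its montage.
; Each answer raises or lowers difficulty, weighted by the question's rating, while entries remain.
; When none remain, WBP_FinalResult shows the difficulty score as the result and dialogue state resets.
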(event OnBeginDialogue(BibleXDialogueTarget)
  (Dialogue|BeginDialogue))

(event OnAnswer(BibleXDialogueTarget)
  (params (IsTrue :type Boolean))
  (Dialogue|ProcessAnswer IsTrue))

(fn ConstructionScript)

(fn BeginDialogue
  (bind _returnvalue (Game|GetPlayerController 0))
  (bind _biblexdialoguetarget (Variables|Default|GetBibleXDialogueTarget))
  (bind _returnvalue_2 (Class|BibleXDialogueTargetComponent|GetDialogueWithinDifficultyLimit _biblexdialoguetarget (Variables|/Script/BibleXDialogue.BibleXDialogueOriginComponent|GetCurrentDifficultyScore (Variables|/Script/BibleXDialogue.BibleXDialogueTargetComponent|GetOriginComponent _biblexdialoguetarget)) true))
  (bind _output_get (Variables|/Script/BibleXDialogue.BibleXDialogueTargetComponent|SetCurrentDialogue (Variables|Default|GetBibleXDialogueTarget) _returnvalue_2))
  (if (> (Utilities|Array|Length (.answers _output_get)) 0)
    (bind _returnvalue_3 (UserInterface|CreateWidget "/Game/Dialogue/Blueprints/UI/WBP_DialogueMain.WBP_DialogueMain_C" 0 (Variables|Default|GetBibleXDialogueTarget) (Utilities|Text|ToText(String) (.dialoguespeakername _output_get)) (Utilities|Text|ToText(String) (.questiontext _output_get)) (.answers _output_get)))
    (Variables|UI|SetMainDialogueWidget _returnvalue_3)
    (UserInterface|Viewport|AddtoViewport _returnvalue_3 0)
    (Input|SetInputModeUIOnly _returnvalue _returnvalue_3 "DoNotLock")
    (Variables|/Script/Engine.PlayerController|SetbShowMouseCursor _returnvalue true)
    (Animation|Montage|MontagePlay (Components|SkeletalMesh|GetAnimInstance (Variables|Default|GetSkeletalMesh)) (.animmontage _output_get) 1.0 "MontageLength" 0.0 true)
    (else
      (Dialogue|ShowResult))))

(fn ProcessAnswer
  (params (IsTrue :type Boolean))
  (Widget|RemovefromParent (Variables|UI|GetMainDialogueWidget))
  (if (> (Utilities|Array|Length (Variables|/Script/BibleXDialogue.BibleXDialogueTargetComponent|GetLocalDataTableNames (Variables|Default|GetBibleXDialogueTarget))) 0)
    (if IsTrue
      (Class|BibleXDialogueOriginComponent|IncreaseDifficulty (Variables|/Script/BibleXDialogue.BibleXDialogueTargetComponent|GetOriginComponent (Variables|Default|GetBibleXDialogueTarget)) (* (Variables|/Script/BibleXDialogue.BibleXDialogueTargetComponent|GetDifficultyGain (Variables|Default|GetBibleXDialogueTarget)) (.difficultyrating (Variables|/Script/BibleXDialogue.BibleXDialogueTargetComponent|GetCurrentDialogue (Variables|Default|GetBibleXDialogueTarget)))))
      (Dialogue|BeginDialogue)
      (else
        (Class|BibleXDialogueOriginComponent|DecreaseDifficulty (Variables|/Script/BibleXDialogue.BibleXDialogueTargetComponent|GetOriginComponent (Variables|Default|GetBibleXDialogueTarget)) (* (Variables|/Script/BibleXDialogue.BibleXDialogueTargetComponent|GetDifficultyGain (Variables|Default|GetBibleXDialogueTarget)) (.difficultyrating (Variables|/Script/BibleXDialogue.BibleXDialogueTargetComponent|GetCurrentDialogue (Variables|Default|GetBibleXDialogueTarget)))))
        (Dialogue|BeginDialogue)))
    (else
      (Dialogue|ShowResult))))

(fn ShowResult
  (bind _returnvalue (UserInterface|CreateWidget "/Game/Dialogue/Blueprints/UI/WBP_FinalResult.WBP_FinalResult_C" 0 (* (Variables|/Script/BibleXDialogue.BibleXDialogueOriginComponent|GetCurrentDifficultyScore (Variables|/Script/BibleXDialogue.BibleXDialogueTargetComponent|GetOriginComponent (Variables|Default|GetBibleXDialogueTarget))) 1e+02)))
  (UserInterface|Viewport|AddtoViewport _returnvalue 0)
  (Class|BibleXDialogueTargetComponent|ResetDialogueState (Variables|Default|GetBibleXDialogueTarget)))